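; BPC_SkillTree is a Blueprint component that holds the skill point balance for a skill tree system.
; GetSkillPoints adds to the balance and SpendSkillPoints subtracts from it without a bounds check, each then firing OnSkillPointsUpdate to notify listeners.
; CheckSkillPoints is a separate query that returns true only when the balance is strictly greater than the queried amount.
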(event EventBeginPlay)

(event EventTick
  (params (DeltaSeconds :type Float%20%28single-precision%29)))

(fn GetSkillPoints
  (params (Amount :type Integer))
  (Variables|Default|SetSkillPoints (+ (Variables|Default|GetSkillPoints) Amount))
  (Default|CallOnSkillPointsUpdate))

(fn SpendSkillPoints
  (params (Amount :type Integer))
  (Variables|Default|SetSkillPoints (- (Variables|Default|GetSkillPoints) Amount))
  (Default|CallOnSkillPointsUpdate))

(fn CheckSkillPoints
  (params (Query :type Integer))
  (return (> (Variables|Default|GetSkillPoints) Query)))
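; BPC_Skills is a component that tracks available skill points and assigned skills for a skill tree.
; Points are awarded with an on-screen message and spent only when the balance covers the amount.
; A map stores a count per skill, and assigning raises it and passes any linked ability to player 0's BPC_Abilities.
; Unassigning only lowers the count, and neither assigning nor unassigning changes the point balance.
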(event EventBeginPlay)

(event EventTick
  (params (DeltaSeconds :type Float%20%28single-precision%29)))

(fn AwardSkillPoint
  (params (SkillPoints :type Integer))
  (Variables|Default|SetSkillPointsAvailable (+ (Variables|Default|GetSkillPointsAvailable) SkillPoints))
  (Development|PrintString "New skill point available!" true true "(R=1.000000,G=0.843620,B=0.000000,A=1.000000)" 5.0))

(fn SpendSkillPoint
  (params (Amount :type Integer))
  (if (CallFunction|QuerySkillPoints Amount)
    (Variables|Default|SetSkillPointsAvailable (- (Variables|Default|GetSkillPointsAvailable) Amount))))

(fn QuerySkillPoints
  (params (Query :type Integer))
  (return (>= (Variables|Default|GetSkillPointsAvailable) Query)))

(fn AssignSkill
  (params (Skill :type DA%20Skill%20Object%20Reference%20%28by%20ref%29))
  (bind _skillsassigned (Variables|Default|GetSkillsAssigned))
  (bind (_value _returnvalue) (Utilities|Map|Find _skillsassigned Skill))
  (Utilities|Map|Add (Variables|Default|GetSkillsAssigned) Skill (Math|Integer|SelectInt (+ _value 1) 1 _returnvalue))
  (bind _ability (Variables|/Game/Blueprints/SkillTree/DA_Skill.DA_Skill_C|GetAbility Skill)
    (:then
      (Default|AddAbility (Actor|GetComponentbyClass (Game|GetPlayerCharacter 0) "/Game/Blueprints/Ability/BPC_Abilities.BPC_Abilities_C") _ability))
    (:else)))

(fn UnassignSkill
  (params (Skill :type DA%20Skill%20Object%20Reference%20%28by%20ref%29))
  (if (> (.Value (CallFunction|QuerySkill Skill)) 0)
    (Utilities|Map|Add (Variables|Default|GetSkillsAssigned) Skill (- (.Value (Utilities|Map|Find (Variables|Default|GetSkillsAssigned) Skill)) 1))))

(fn QuerySkill
  (params (Skill :type DA%20Skill%20Object%20Reference%20%28by%20ref%29))
  (bind _skillsassigned (Variables|Default|GetSkillsAssigned))
  (bind (_value _returnvalue) (Utilities|Map|Find _skillsassigned Skill))
  (return _value _returnvalue))